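; BP_Ghost1 is a ghost pawn that wanders and moves toward the player on sight.
; It loops an idle bobbing animation and chains AI moves to random nearby navigable points, picking another only when a move succeeds.
; Pawn Sensing redirects it toward a seen first-person character unless that player is invisible.
; Its Any Damage event calls Apply Damage with no target connected.
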(event OnSeePawn(PawnSensing)
  (params (Pawn :type Pawn%20Object%20Reference))
  (bind _asbp_first_person_character (Utilities|Casting|CastToBP_FirstPersonCharacter Pawn))
  (if (== (Variables|/Game/FirstPerson/Blueprints/BP_FirstPersonCharacter.BP_FirstPersonCharacter_C|GetisInvisible _asbp_first_person_character) false)
    (AI|AIMoveTo self "0, 0, 0" _asbp_first_person_character 1e+02 false)))

(event Custom|MoveToRandomLocation
  (Components|Animation|PlayAnimation (Variables|Character|GetMesh) "/Game/Fab/Dark_Big_Ghost__LITE_/big_ghost_lite_Anim_idle_up_down.big_ghost_lite_Anim_idle_up_down" true)
  (bind _randomlocation (Class|NavigationSystemV1|GetRandomLocationinNavigableRadius (Transformation|GetActorLocation) 5e+02 0 0))
  (AI|AIMoveTo self _randomlocation 0 5.0 false
    (:OnSuccess
      (CallFunction|MovetoRandomLocation))))

(event EventBeginPlay
  (CallFunction|MovetoRandomLocation))

(event Game|Damage|EventAnyDamage
  (params (Damage :type Float%20%28single-precision%29) (DamageType :type Damage%20Type%20Object%20Reference) (InstigatedBy :type Controller%20Object%20Reference) (DamageCauser :type Actor%20Object%20Reference))
  (Game|Damage|ApplyDamage 0 1e+01 0 0))

(fn ConstructionScript)