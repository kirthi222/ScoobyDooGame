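; Ghost AI pawn that wanders at random and pursues pawns it sees.
; It loops a floating idle animation and chains AI moves to random navigable points around its current location.
; PawnSensing sightings start a move toward the seen pawn, while a retriggerable delay resumes wandering shortly after sightings stop.
; The AnyDamage handler calls ApplyDamage with no target set.
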(event OnSeePawn(PawnSensing)
  (params (Pawn :type Pawn%20Object%20Reference))
  (Utilities|FlowControl|Sequence
    (:then_0
      (AI|AIMoveTo self "0, 0, 0" Pawn 5.0 false))
    (:then_1
      (Utilities|FlowControl|RetriggerableDelay 1.0)
      (CallFunction|MovetoRandomLocation))))

(event Custom|MoveToRandomLocation
  (Components|Animation|PlayAnimation (Variables|Character|GetMesh) "/Game/Fab/Dark_Big_Ghost__LITE_/big_ghost_lite_Anim_idle_up_down.big_ghost_lite_Anim_idle_up_down" true)
  (bind _randomlocation (Class|NavigationSystemV1|GetRandomLocationinNavigableRadius (Transformation|GetActorLocation) 5e+02 0 0))
  (AI|AIMoveTo self _randomlocation 0 5.0 false
    (:OnSuccess
      (CallFunction|MovetoRandomLocation))))

(event EventBeginPlay
  (CallFunction|MovetoRandomLocation))

(event Game|Damage|EventAnyDamage
  (params (Damage :type Float%20%28single-precision%29) (DamageType :type Damage%20Type%20Object%20Reference) (InstigatedBy :type Controller%20Object%20Reference) (DamageCauser :type Actor%20Object%20Reference))
  (Game|Damage|ApplyDamage 0 1e+01 0 0))

(fn ConstructionScript)